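; BP_ScreamJamGM is the ScreamJam game mode, holding the win and lose endings.
; Each event plays its own sound, adds a fade-to-black widget and disables input on the player's BP_ScreamJamCharacter.
; After a delay, losing opens MainMap while winning quits the game.
; Nothing in this graph calls either event, so both rely on outside triggers.
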(event EventLoseCondition
  (Audio|PlaySound2D "/Game/Audio/AlexTalking/ScreamJam_LoseCondition.ScreamJam_LoseCondition" 1.0 1.0 0.0 0 0)
  (bind _returnvalue (UserInterface|CreateWidget "/Game/Blueprints/Widgets/WBP_FadeOutToBlack.WBP_FadeOutToBlack_C" (Game|GetPlayerController 0)))
  (UserInterface|Viewport|AddtoViewport _returnvalue 0)
  (bind _asbp_scream_jam_character (Utilities|Casting|CastToBP_ScreamJamCharacter (Game|GetPlayerCharacter 0)))
  (Variables|/Script/ScreamJam2023.ScreamJamCharacter|SetbCanReceiveInput _asbp_scream_jam_character false)
  (Utilities|FlowControl|Delay 1e+01)
  (Game|OpenLevel(byName) "MainMap"))

(event EventWinCondition
  (Audio|PlaySound2D "/Game/Audio/AlexTalking/ScreamJam_WinCondition.ScreamJam_WinCondition" 1.0 1.0 0.0 0 0)
  (bind _returnvalue (UserInterface|CreateWidget "/Game/Blueprints/Widgets/WBP_FadeOutToBlack.WBP_FadeOutToBlack_C" (Game|GetPlayerController 0)))
  (UserInterface|Viewport|AddtoViewport _returnvalue 0)
  (Utilities|Casting|CastToBP_ScreamJamCharacter (Game|GetPlayerCharacter 0))
  (Variables|/Script/ScreamJam2023.ScreamJamCharacter|SetbCanReceiveInput (stale EventLoseCondition _asbp_scream_jam_character) false)
  (Utilities|FlowControl|Delay 8.0)
  (Game|QuitGame 0 "Quit" false))

(fn ConstructionScript)