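; BP_ExplainInteract is a one-time trigger volume that shows an interaction explanation to the player.
; When BP_ScreamJamCharacter overlaps BoxCollider, it disables that character's input, plays audio and adds WBP_ExplainInteract to the viewport.
; After a four-second delay it restores input and only then sets the Occured flag that blocks later triggers.
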(event OnComponentBeginOverlap(BoxCollider)
  (params (OverlappedComponent :type Primitive%20Component%20Object%20Reference) (OtherActor :type Actor%20Object%20Reference) (OtherComp :type Primitive%20Component%20Object%20Reference) (OtherBodyIndex :type Integer) (bFromSweep :type Boolean) (SweepResult :type Hit%20Result%20Structure%20%28by%20ref%29))
  (if (not (Variables|Default|GetbOccured))
    (bind _asbp_scream_jam_character (Utilities|Casting|CastToBP_ScreamJamCharacter OtherActor))
    (Variables|/Script/ScreamJam2023.ScreamJamCharacter|SetbCanReceiveInput _asbp_scream_jam_character false)
    (Class|PlayAudioOnceinVolume|PlayAudio)
    (bind _returnvalue (UserInterface|CreateWidget "/Game/Blueprints/Widgets/WBP_ExplainInteract.WBP_ExplainInteract_C" (Game|GetPlayerController 0)))
    (UserInterface|Viewport|AddtoViewport _returnvalue 0)
    (Utilities|FlowControl|Delay 4.0)
    (Variables|/Script/ScreamJam2023.ScreamJamCharacter|SetbCanReceiveInput _asbp_scream_jam_character true)
    (Variables|Default|SetbOccured true)))

(event EventBeginPlay)

(event Collision|EventActorBeginOverlap
  (params (OtherActor :type Actor%20Object%20Reference)))

(event EventTick
  (params (DeltaSeconds :type Float%20%28single-precision%29)))

(fn ConstructionScript)