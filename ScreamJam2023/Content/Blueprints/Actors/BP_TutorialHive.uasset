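; BP_TutorialHive is the interactable hive in the tutorial whose destruction ends it and sends the player to the main map.
; Its box collider shows a prompt widget component while the ScreamJam character overlaps it and hides it on exit.
; On InteractEvent it waits briefly, removes the collider, adds a fade-to-black widget, plays the nest-destroyed sound, then opens MainMap after a delay.
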(event OnComponentBeginOverlap(BoxCollider)
  (params (OverlappedComponent :type Primitive%20Component%20Object%20Reference) (OtherActor :type Actor%20Object%20Reference) (OtherComp :type Primitive%20Component%20Object%20Reference) (OtherBodyIndex :type Integer) (bFromSweep :type Boolean) (SweepResult :type Hit%20Result%20Structure%20%28by%20ref%29))
  (Utilities|Casting|CastToBP_ScreamJamCharacter OtherActor)
  (Rendering|SetVisibility (Variables|Default|GetWidget) true false))

(event OnComponentEndOverlap(BoxCollider)
  (params (OverlappedComponent :type Primitive%20Component%20Object%20Reference) (OtherActor :type Actor%20Object%20Reference) (OtherComp :type Primitive%20Component%20Object%20Reference) (OtherBodyIndex :type Integer))
  (Utilities|Casting|CastToBP_ScreamJamCharacter OtherActor)
  (Rendering|SetVisibility (Variables|Default|GetWidget) false false))

(event EventInteractEvent
  (Utilities|FlowControl|Delay 0.3)
  (Utilities|IsValid self
    (:Is%20Valid
      (Components|DestroyComponent (Variables|Default|GetBoxCollider))
      (bind _returnvalue (UserInterface|CreateWidget "/Game/Blueprints/Widgets/WBP_FadeOutToBlack.WBP_FadeOutToBlack_C" (Game|GetPlayerController 0)))
      (UserInterface|Viewport|AddtoViewport _returnvalue 0)
      (Audio|PlaySound2D "/Game/Audio/AlexTalking/ScreamJamTutorialNestDestroyed.ScreamJamTutorialNestDestroyed" 1.0 1.0 0.0 0 0)
      (Utilities|FlowControl|Delay 5.0)
      (Game|OpenLevel(byName) "MainMap"))))

(fn ConstructionScript)