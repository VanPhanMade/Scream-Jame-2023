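; Destructible nest objective actor for the ScreamJam game mode that counts toward victory.
; It registers with BP_ScreamJamGM on BeginPlay, and on interaction waits briefly, tells the game mode to remove it and check victory, then destroys itself.
; A box collider toggles a widget's visibility while the ScreamJam character overlaps it.
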(event OnComponentBeginOverlap(BoxCollider)
  (params (OverlappedComponent :type Primitive%20Component%20Object%20Reference) (OtherActor :type Actor%20Object%20Reference) (OtherComp :type Primitive%20Component%20Object%20Reference) (OtherBodyIndex :type Integer) (bFromSweep :type Boolean) (SweepResult :type Hit%20Result%20Structure%20%28by%20ref%29))
  (Utilities|Casting|CastToBP_ScreamJamCharacter OtherActor)
  (Rendering|SetVisibility (Variables|Default|GetWidget) true false))

(event OnComponentEndOverlap(BoxCollider)
  (params (OverlappedComponent :type Primitive%20Component%20Object%20Reference) (OtherActor :type Actor%20Object%20Reference) (OtherComp :type Primitive%20Component%20Object%20Reference) (OtherBodyIndex :type Integer))
  (Utilities|Casting|CastToBP_ScreamJamCharacter OtherActor)
  (Rendering|SetVisibility (Variables|Default|GetWidget) false false))

(event EventBeginPlay
  (bind _asbp_scream_jam_gm (Utilities|Casting|CastToBP_ScreamJamGM (Game|GetGameMode)))
  (Class|ScreamJam2023GameModeBase|RegisterNest _asbp_scream_jam_gm))

(event EventInteractEvent
  (Utilities|FlowControl|Delay 0.3)
  (Utilities|IsValid self
    (:Is%20Valid
      (Class|ScreamJam2023GameModeBase|RemoveNestandCheckVictory (stale EventBeginPlay _asbp_scream_jam_gm))
      (Actor|DestroyActor))))

(fn ConstructionScript)